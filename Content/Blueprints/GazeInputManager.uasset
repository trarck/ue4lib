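; Actor that manages gaze-based pointer input, feeding a GazeInput component into gaze processing and widget interaction.
; On BeginPlay, if a player pawn exists, GazeInput ignores the pawn and itself, ticks in PostUpdateWork, and registers with GazeProcessor and WidgetInputManager.
; It also enables player controller input so the Fire action presses and releases GazeInput's pointer key.
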(event EventBeginPlay
  (bind _returnvalue (Game|Player|GetPlayerPawn 0))
  (bind _gazeinput (Variables|Default|GetGazeInput))
  (if (Utilities|IsValid _returnvalue)
    (Class|RayInput|AddIgnoreActor _gazeinput _returnvalue)
    (Class|RayInput|AddIgnoreActor _gazeinput self)
    (Components|Tick|SetTickGroup (Variables|Default|GetGazeInput) "TG_PostUpdateWork")
    (Class|GazeProcessor|RegisterProcess (Variables|Default|GetGazeProcessor) (Variables|Default|GetGazeInput))
    (Class|WidgetInputManagerComponent|RegisterProcess (Variables|Default|GetWidgetInputManager) (Variables|Default|GetGazeInput))
    (Input|EnableInput (Game|GetPlayerController 0))))

(event Collision|EventActorBeginOverlap
  (params (OtherActor :type Actor%20Object%20Reference)))

(event EventTick
  (params (DeltaSeconds :type Float%20%28single-precision%29)))

(event Input|ActionEvents|InputActionFire
  (params (Key :type Key%20Structure :default "AnyKey"))
  (bind _gazeinput (Variables|Default|GetGazeInput))
  (:Pressed
    (Class|RayInput|PressPointerKey _gazeinput Key))
  (:Released
    (Class|RayInput|ReleasePointerKey _gazeinput Key)))

(fn ConstructionScript)