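; Actor that provides gaze-based selection input and forwards button presses through its GazeInput component.
; On BeginPlay, if a player pawn exists, GazeInput ignores that pawn and the actor, ticks in PostUpdateWork, and registers with GazeSelectProcessor and WidgetInteractionManager.
; It then enables player input, so the Fire action drives pointer key press and release.
; The G key is forwarded as a keyboard key, with a debug "Hello" print on press.
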(event EventBeginPlay
  (bind _returnvalue (Game|Player|GetPlayerPawn 0))
  (bind _gazeinput (Variables|Default|GetGazeInput))
  (if (Utilities|IsValid _returnvalue)
    (Class|RayInput|AddIgnoreActor _gazeinput _returnvalue)
    (Class|RayInput|AddIgnoreActor _gazeinput self)
    (Components|Tick|SetTickGroup (Variables|Default|GetGazeInput) "TG_PostUpdateWork")
    (Class|GazeSelectProcessor|RegisterProcess (Variables|Default|GetGazeSelectProcessor) (Variables|Default|GetGazeInput))
    (Class|WidgetInteractionManagerComponent|RegisterProcess (Variables|Default|GetWidgetInteractionManager) (Variables|Default|GetGazeInput))
    (Input|EnableInput (Game|GetPlayerController 0))))

(event Input|ActionEvents|InputActionFire
  (params (Key :type Key%20Structure :default "AnyKey"))
  (bind _gazeinput (Variables|Default|GetGazeInput))
  (:Pressed
    (Class|RayInput|PressPointerKey _gazeinput Key))
  (:Released
    (Class|RayInput|ReleasePointerKey _gazeinput Key)))

(event Input|KeyboardEvents|G
  (params (Key :type Key%20Structure :default "AnyKey"))
  (bind _gazeinput (Variables|Default|GetGazeInput))
  (:Pressed
    (Development|PrintString "Hello")
    (Class|RayInput|PressKey _gazeinput Key false))
  (:Released
    (Class|RayInput|ReleaseKey _gazeinput Key)))

(fn ConstructionScript)