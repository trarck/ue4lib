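; Test actor that wires a GazeInput component to a GazePointer for gaze ray input.
; On BeginPlay, if the player pawn is valid, the gaze input ignores that pawn and itself, ticks in PostUpdateWork, and is registered as a process on the pointer.
; The ray callback is empty; disconnected nodes for moving something to the hit point or ray end never run.
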(event OnProcessRay(GazeInput)
  (params (bHit :type Boolean) (Start :type Vector%20%28by%20ref%29) (End :type Vector%20%28by%20ref%29) (HitResult :type Hit%20Result%20Structure%20%28by%20ref%29) (bBeginHit :type Boolean) (bHaveRay :type Boolean)))

(event EventBeginPlay
  (bind _returnvalue (Game|Player|GetPlayerPawn 0))
  (bind _gazeinput (Variables|Default|GetGazeInput))
  (if (Utilities|IsValid _returnvalue)
    (Class|RayInput|AddIgnoreActor _gazeinput _returnvalue)
    (Class|RayInput|AddIgnoreActor _gazeinput self)
    (Components|Tick|SetTickGroup (Variables|Default|GetGazeInput) "TG_PostUpdateWork")
    (Class|GazePointer|RegisterProcess (Variables|Default|GetGazePointer) (Variables|Default|GetGazeInput))))

(event Collision|EventActorBeginOverlap
  (params (OtherActor :type Actor%20Object%20Reference)))

(event EventTick
  (params (DeltaSeconds :type Float%20%28single-precision%29)))

(fn ConstructionScript)