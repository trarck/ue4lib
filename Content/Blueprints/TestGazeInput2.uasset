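; Test actor that sets up gaze-based input and lets the Fire action act as an Enter key press for UMG.
; On BeginPlay, if the player pawn is valid, GazeInput ignores the pawn and itself, ticks in PostUpdateWork and registers with GazeProcessor, then the actor enables player input.
; Fire press and release forward Enter key down and up events to GazeInput.
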(event EventBeginPlay
  (bind _returnvalue (Game|Player|GetPlayerPawn 0))
  (bind _gazeinput (Variables|Default|GetGazeInput))
  (if (Utilities|IsValid _returnvalue)
    (Class|RayInput|AddIgnoreActor _gazeinput _returnvalue)
    (Class|RayInput|AddIgnoreActor _gazeinput self)
    (Components|Tick|SetTickGroup (Variables|Default|GetGazeInput) "TG_PostUpdateWork")
    (Class|GazeProcessor|RegisterProcess (Variables|Default|GetGazeProcessor) (Variables|Default|GetGazeInput))
    (Input|EnableInput (Game|GetPlayerController 0))))

(event Collision|EventActorBeginOverlap
  (params (OtherActor :type Actor%20Object%20Reference)))

(event EventTick
  (params (DeltaSeconds :type Float%20%28single-precision%29)))

(event Input|ActionEvents|InputActionFire
  (params (Key :type Key%20Structure :default "AnyKey"))
  (bind _gazeinput (Variables|Default|GetGazeInput))
  (:Pressed
    ;[1 1 1] Fire Key to Enter Key support by umg
    (bind _returnvalue (Class|YHInputUtil|GetInputKey "Enter"))
    (Class|RayInput|HandleKeyDown _gazeinput _returnvalue))
  (:Released
    (bind _returnvalue_2 (Class|YHInputUtil|GetInputKey "Enter"))
    (Class|RayInput|HandleKeyUp _gazeinput _returnvalue_2)))

(fn ConstructionScript)