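; PossessComponent is a Blueprint component that directs the first player's input to a target, using an input component stack instead of pawn possession.
; Possess checks for a repeat target, releases the old one via UnPossess, then creates an InputComponent owned by the new target and pushes it onto PlayerController 0.
; UnPossess pops that InputComponent and clears both references, with debug prints reporting results.
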(event EventBeginPlay)

(event EventTick
  (params (DeltaSeconds :type Float%20%28single-precision%29)))

(fn Possess
  (params (Target :type Pawn%20Object%20Reference))
  ;[1 1 1] Check Target
  (if (== Target (Variables|Default|GetTarget))
    (Development|PrintString "Target possessing")
    (else
      (if (Utilities|IsValid (Variables|Default|GetTarget))
        (CallFunction|UnPossess))
      (bind _output_get (Variables|Default|SetTarget Target))
      (if (Utilities|IsValid _output_get)
        ;[1 1 1] Do Controll
        (bind _returnvalue (Class|InputUtil|CreateInputComponent (Variables|Default|GetTarget) "InputComponent" false))
        (bind _output_get_2 (Variables|Default|SetInputComponent _returnvalue))
        (Class|InputUtil|PushInputComponent (Game|GetPlayerController 0) _output_get_2)
        (Development|PrintString "Possess Success")
        (else
          (Development|PrintString "Possess No Target"))))))

(fn UnPossess
  (if (Utilities|IsValid (Variables|Default|GetTarget))
    _
    (else
      (Development|PrintString "UnPossess No Target")))
  (if (Utilities|IsValid (Variables|Default|GetInputComponent))
    (Class|InputUtil|PopInputComponent (Game|GetPlayerController 0) (Variables|Default|GetInputComponent))
    (Variables|Default|SetInputComponent 0)
    (else
      (Development|PrintString "UnPossess No InputComponent")))
  (Variables|Default|SetTarget 0))